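; HexGrid_BP is an actor that builds a grid of static mesh tiles, laid out as a hex grid, in its construction script.
; Nested loops over GridX and GridY place one mesh component per cell, shifting every odd column along Y by Offset to stagger the layout.
; Each tile gets two random scalar material parameters, RNG1 and RNG2, for per-tile variation.
; The event graph is empty, and the extra function and macro graphs appear to be leftover scaffolding.
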(event EventBeginPlay)

(event Collision|EventActorBeginOverlap
  (params (OtherActor :type Actor%20Object%20Reference)))

(event EventTick
  (params (DeltaSeconds :type Float%20%28single-precision%29)))

(fn ConstructionScript
  (for _index (range 0 (Variables|Default|GetGrid%20X))
    (for _index_2 (range 0 (Variables|Default|GetGrid%20Y))
      (bind _returnvalue (AddComponent|AddStaticMeshComponent false (Math|Transform|MakeTransform (Math|Vector|SelectVector (Math|Vector|MakeVector (* _index (* (Variables|Default|GetSpacing%20X) 9e+01)) (* _index_2 (Variables|Default|GetSpacing%20Y)) 0.0) (Math|Vector|MakeVector (* _index (* (Variables|Default|GetSpacing%20X) 9e+01)) (+ (Variables|Default|GetOffset) (* _index_2 (Variables|Default|GetSpacing%20Y))) 0.0) (== (Math|Integer|%(Integer) _index 2) 0)) "0, 0, 0" "1.000000,1.000000,1.000000")))
      (Rendering|Material|SetScalarParameterValueonMaterials _returnvalue "RNG2" (Math|Random|RandomFloatinRange 0.0 1e+03))
      (Rendering|Material|SetScalarParameterValueonMaterials _returnvalue "RNG1" (Math|Random|RandomFloatinRange 0.0 7e+02)))))

(fn NewFunction0
  (|CollapseGraph_0))